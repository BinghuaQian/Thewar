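; A function library of helpers for the boss enemy, providing a percentage chance roll and a movement speed setter.
; Maybe clamps its input to a 0–100 percentage and compares it to a random float, returning true with roughly that probability.
; SetSpeed casts the target to BossBP2 and sets its max walk speed from the boss's walk speed, run speed or a supplied value, chosen by speed type.
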(fn `Maybe`
  (params (Num :type "Float (double-precision)"))
  (returns (Return :type Boolean))
  (return (> (`KismetMathLibrary.FClamp` Num 0.0 100.0) (`KismetMathLibrary.RandomFloatInRange` 0.0 100.0))))

(fn `SetSpeed`
  (params (Target :type "Character Object Reference") (Speed :type "Float (double-precision)") (`Speed Type` :type "/Game/enmy/b/Enum/SpeedType Enum" :default "NewEnumerator0"))
  (bind _asboss_bp2 (cast `/Game/enmy/b/Boss/BossBP2` Target))
  (set `CharacterMovementComponent.MaxWalkSpeed` (select `/Game/enmy/b/Enum/SpeedType` `Speed Type` :`NewEnumerator0` (`/Game/enmy/b/Boss/BossBP2.WalkSpeed` _asboss_bp2) :`NewEnumerator1` (`/Game/enmy/b/Boss/BossBP2.RunSpeed` _asboss_bp2) :`NewEnumerator2` Speed) (`Character.CharacterMovement` _asboss_bp2)))