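; BP_flySword is a flying-sword projectile actor, filed with the boss enemy assets.
; The construction script gives its ProjectileMovement a fixed initial speed and a randomized max speed, and BeginPlay caches the spawn location.
; A Timeline is built to raise the sword vertically, then activate projectile movement after a short delay, but nothing triggers it, so that sequence never runs.
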(event `self.ReceiveBeginPlay`
  (set `self.InitLocation` (`self.K2_GetActorLocation`)))

(fn `UserConstructionScript`
  (bind _projectilemovement (`self.ProjectileMovement`))
  (set `ProjectileMovementComponent.InitialSpeed` 1200.0 _projectilemovement)
  (set `ProjectileMovementComponent.MaxSpeed` (`KismetMathLibrary.RandomFloatInRange` 1200.0 2000.0) _projectilemovement))