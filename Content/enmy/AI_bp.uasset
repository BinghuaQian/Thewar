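; Zombie enemy that loses health to magic projectiles and equipped-player contact, showing health on a widget bar updated every Tick.
; Magic hits spawn explosions; capsule contact damages it when the Hit flag is set.
; Its sphere overlap drains player BloodValue once and loops the attack montage by timer until overlap ends.
; Death awards GameMode experience, handles level-ups with a widget and player stat boosts, then destroys the actor.
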(event `self.ReceiveBeginPlay`)

(event `self.ReceiveActorBeginOverlap`
  (params (OtherActor :type "Actor Object Reference"))
  (bind _asmagic_point (cast `/Game/Effect/magic/magicPoint` OtherActor))
  (`KismetSystemLibrary.PrintString` "hit")
  (`GameplayStatics.SpawnEmitterAtLocation` "/Game/StarterContent/Particles/P_Explosion.P_Explosion" (`self.K2_GetActorLocation` _asmagic_point))
  (bind _output_get (set `self.Health` (- (`self.Health`) 0.25)))
  (if (<= _output_get 0.0)
    (`self.Death`)
    (`self.K2_DestroyActor` _asmagic_point)
    (else
      (`self.K2_DestroyActor` OtherActor))))

(event `self.CapsuleComponent.OnComponentBeginOverlap`
  (params (OverlappedComponent :type "PrimitiveComponent Object Reference") (OtherActor :type "Actor Object Reference") (OtherComp :type "PrimitiveComponent Object Reference") (OtherBodyIndex :type Integer) (bFromSweep :type Boolean) (SweepResult :type "HitResult Structure (by ref)"))
  (bind _asplayer (cast `/Game/human/player` OtherActor))
  (if (`/Game/human/player.euip?` _asplayer)
    (if (`self.hit?`)
      (`KismetSystemLibrary.PrintString` "het")
      (bind _output_get (set `self.Health` (- (`self.Health`) 0.25)))
      (if (<= _output_get 0.0)
        (`self.Death`))
      (else
        (set `self.hit?` false)
        (`KismetSystemLibrary.Delay` 1.0)
        (set `self.hit?` true)))))

(event `loop`
  (bind _returnvalue (`AnimInstance.Montage_Play` (`SkeletalMeshComponent.GetAnimInstance` (`self.Mesh`)) "/Game/enmy/Animation/Zombie_Attack_Montage.Zombie_Attack_Montage" 1.5 "MontageLength" 0.0 true :!label _label))
  (bind _returnvalue_2 (`KismetSystemLibrary.K2_SetTimerDelegate` (delegate `loop`) _returnvalue true)))

(event `self.Sphere.OnComponentBeginOverlap`
  (params (OverlappedComponent :type "PrimitiveComponent Object Reference") (OtherActor :type "Actor Object Reference") (OtherComp :type "PrimitiveComponent Object Reference") (OtherBodyIndex :type Integer) (bFromSweep :type Boolean) (SweepResult :type "HitResult Structure (by ref)"))
  (bind _asplayer (cast `/Game/human/player` OtherActor))
  (set `/Game/human/player.BloodValue` (- (`/Game/human/player.BloodValue` _asplayer) 5.0) _asplayer)
  (goto _label))

(event `self.Sphere.OnComponentEndOverlap`
  (params (OverlappedComponent :type "PrimitiveComponent Object Reference") (OtherActor :type "Actor Object Reference") (OtherComp :type "PrimitiveComponent Object Reference") (OtherBodyIndex :type Integer))
  (cast `/Game/human/player` OtherActor)
  (`KismetSystemLibrary.K2_ClearAndInvalidateTimerHandle` (stale `loop` _returnvalue_2)))

(event `self.ReceiveTick`
  (params (DeltaSeconds :type "Float (single-precision)"))
  (bind _asaihealth (cast `/Game/enmy/AIhealth` (`WidgetComponent.GetWidget` (`self.Widget`))))
  (`ProgressBar.SetPercent` (`/Game/enmy/AIhealth.health_Ai` _asaihealth) (`self.Health`)))

(fn `Death`
  (bind _asthird_person_game_mode (cast `/Game/human/ThirdPersonGameMode` (`GameplayStatics.GetGameMode`)))
  (bind _output_get (set `/Game/human/ThirdPersonGameMode.experience` (+ (`/Game/human/ThirdPersonGameMode.experience` _asthird_person_game_mode) 1) _asthird_person_game_mode))
  (if (>= _output_get (`/Game/human/ThirdPersonGameMode.maxExperience` _asthird_person_game_mode))
    (set `/Game/human/ThirdPersonGameMode.level` (+ (`/Game/human/ThirdPersonGameMode.level` _asthird_person_game_mode) 1) _asthird_person_game_mode)
    (set `/Game/human/ThirdPersonGameMode.experience` 0 _asthird_person_game_mode)
    (set `/Game/human/ThirdPersonGameMode.maxExperience` (* (`/Game/human/ThirdPersonGameMode.maxExperience` _asthird_person_game_mode) 2) _asthird_person_game_mode)
    (bind _returnvalue (`|CreateWidget` "/Game/ThirdPersonBP/UI/levelUp.levelUp_C"))
    (`UserWidget.AddToViewport` _returnvalue 0)
    (bind _asplayer (cast `/Game/human/player` (`GameplayStatics.GetPlayerCharacter` 0)))
    (set `/Game/human/player.energyMax` (* (`/Game/human/player.energyMax` _asplayer) 1.2) _asplayer)
    (set `/Game/human/player.energy` (* (`/Game/human/player.energy` _asplayer) 1.2) _asplayer)
    (set `/Game/human/player.healthMax` (* (`/Game/human/player.healthMax` _asplayer) 1.2) _asplayer)
    (set `/Game/human/player.health` (* (`/Game/human/player.BloodValue` _asplayer) 1.2) _asplayer))
  (`self.K2_DestroyActor`))

(fn `Take Damage`
  (`GameplayStatics.SpawnEmitterAtLocation` "/Game/StarterContent/Particles/P_Explosion.P_Explosion"))

(fn `UserConstructionScript`)