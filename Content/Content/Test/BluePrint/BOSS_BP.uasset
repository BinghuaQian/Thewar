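; Boss actor Blueprint providing melee attack tracing, movement helpers and health regeneration.
; AttackTrace runs a debug-drawn box trace between two weapon sockets, without acting on the result.
; DodgeMove and BaseMove use timelines to sweep the boss backward or, after a delay, along its forward vector for attack displacement.
; After a retriggerable delay, huixue sets a blackboard flag and starts a looping timer that restores clamped HP while the flag holds.
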(event `AttackTrace`
  ;[1 1 1] 攻击检测
  (`KismetSystemLibrary.BoxTraceSingle` :`Start` (`SceneComponent.GetSocketLocation` (`self.Weapon`) "Socket1") :`End` (`SceneComponent.GetSocketLocation` (`self.Weapon`) "Socket2") :`HalfSize` (0.5 0.5 0.5) :`TraceChannel` "TraceTypeQuery1" :`DrawDebugType` "ForDuration"))

(event `Dodge Move`
  ;[1 1 1] 后撤步的移动
  (set `self.CurrentLoc` (`self.K2_GetActorLocation`))
  (bind (_direction `_新建轨迹_0`) (`Timeline|时间轴_0` :!via `PlayFromStart`)
    (:`Update`
      (`self.K2_SetActorLocation` (`KismetMathLibrary.VLerp` (`self.CurrentLoc`) (+ (`self.CurrentLoc`) (* (`self.GetActorForwardVector`) -300.0)) `_新建轨迹_0`) true))))

(event `BaseMove`
  (params (Duration :type "Float (double-precision)") (Stength :type "Float (double-precision)"))
  ;[1 1 1] 基本的移动，用于攻击上的位移
  (`KismetSystemLibrary.Delay` Duration)
  (set `self.CurrentLoc` (`self.K2_GetActorLocation`))
  (bind (_direction `_新建轨迹_0`) (`Timeline|时间轴_1` :!via `PlayFromStart`)
    (:`Update`
      (`self.K2_SetActorLocation` (`KismetMathLibrary.VLerp` (`self.CurrentLoc`) (+ (`self.CurrentLoc`) (* (`self.GetActorForwardVector`) Stength)) `_新建轨迹_0`) true))))

(event `huixue`
  ;[1 1 1] 呼吸回血条件
  (`KismetSystemLibrary.RetriggerableDelay` 5.0)
  (`BlackboardComponent.SetValueAsBool` (`AIBlueprintHelperLibrary.GetBlackboard` self) "huixue" true)
  (`KismetSystemLibrary.K2_SetTimerDelegate` (delegate `jia xue`) 1.0 true))

(event `jia xue`
  ;[1 1 1] 呼吸回血具体
  (if (`BlackboardComponent.GetValueAsBool` (`AIBlueprintHelperLibrary.GetBlackboard` self) "huixue")
    (bind _output_get (set `self.HP` (`KismetMathLibrary.FClamp` (+ (`self.HP`) 5.0) 0.0 100.0)))
    (`KismetSystemLibrary.PrintString` (`KismetStringLibrary.Conv_DoubleToString` _output_get))))

(fn `UserConstructionScript`)