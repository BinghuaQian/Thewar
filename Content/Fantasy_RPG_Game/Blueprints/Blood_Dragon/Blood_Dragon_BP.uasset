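; Blood Dragon enemy character that plays a detection animation, chases the player, attacks with bites and fire breath, and takes sword, bomb and power-attack damage.
; A self-calling Initialize loop drives AI movement and randomly picks bite, grounded fire or flying fire, using DoOnce gates with delayed resets as cooldowns.
; Bite-box overlaps and fire particle collisions damage the player, with random spark spawns.
; Death awards XP, removes the health widget and ragdolls the mesh.
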(event `Attach_Dragon_Bite_Box`
  ;[1 1 1] Attach_Dragon_Bite_Collision_Box
  (`/Engine/EditorBlueprintResources/StandardMacros.DoOnce` false
    (:`Completed`
      (`SceneComponent.K2_AttachToComponent` (`self.Dragon_Bite_Collision_Box`) (`self.Mesh`) "Fire_Socket" "KeepWorld" "KeepWorld" "KeepWorld" true)
      (`KismetSystemLibrary.Delay` 5.0)
      (set `self.Can_Follow_Player` true))))

(event `Dragon_Bite`
  ;[1 1 1] Bite
  (if (not (`self.Dead`))
    (`self.Look_At_Player`)
    (`KismetSystemLibrary.Delay` 0.3)
    (set `self.Can_Look_At_Player` false)
    (set `self.Bite` true)
    (`KismetSystemLibrary.Delay` 2.0)
    (set `self.Bite` false)
    (`KismetSystemLibrary.Delay` 3.2)
    (set `self.Can_Look_At_Player` true)
    (`self.Reset_Do_once`)))

(event `Reset_Do_once`
  ;[1 1 1] Randomly_Switch_Between_Call_Bite or Breath_Fire_While_Flying
  (set `self.Can_Follow_Player` true)
  (goto _label_2 :!via `Reset`))

(event `BreathFire_Flying`
  (bind _dragon_fire (`self.Dragon_Fire`))
  (bind _charactermovement (`self.CharacterMovement`))
  ;[1 1 1] Breath_Fire_Flying
  (`/Engine/EditorBlueprintResources/StandardMacros.DoOnce` false :!label _label
    (:`Completed`
      (if (not (`self.Dead`))
        (set `self.Can_Follow_Player` false)
        (set `self.Breath_Fire_Flying` true)
        (set `self.Can_Look_At_Player` false)
        (`|ExecutionSequence`
          (:`then_0`
            (`KismetSystemLibrary.Delay` 9.0)
            (`ActorComponent.Activate` _dragon_fire true)
            (`SceneComponent.K2_AttachToComponent` _dragon_fire (`self.Mesh`) "Fire_Socket" "KeepRelative" "KeepRelative" "KeepRelative" true)
            (`KismetSystemLibrary.Delay` 7.0)
            (`ActorComponent.Deactivate` _dragon_fire)
            (set `self.Can_Follow_Player` true)
            (`KismetSystemLibrary.Delay` 15.0)
            (`self.Reset_Do_Once_3`))
          (:`then_1`
            (`CharacterMovementComponent.SetMovementMode` _charactermovement "MOVE_Flying" 0)
            (`KismetSystemLibrary.Delay` 17.5)
            (set `self.Breath_Fire_Flying` false)
            (`PrimitiveComponent.SetCollisionEnabled` (`self.CapsuleComponent`) "QueryAndPhysics")
            (set `self.Can_Look_At_Player` false)
            (`self.Reset_Do_once`)
            (`CharacterMovementComponent.SetMovementMode` _charactermovement "MOVE_Walking" 0)
            (set `self.Can_Follow_Player` true)
            (`self.Initialize`)
            (`self.Look_At_Player`)
            (`self.Reset_Do_once`)))))))

(event `Reset_Do_Once_3`
  ;[1 1 1] Breath_Fire_Flying
  (goto _label :!via `Reset`))

(event `Follow_Player`
  ;[1 1 1] Follow_Player
  (if (`self.Dead`)
    _
    (elif (not (`self.Breath_Fire_Grounded`))
      (bind _aswarrior_character_bp (cast `/Game/Fantasy_RPG_Game/Blueprints/Warrior/Warrior_Character_BP` (`GameplayStatics.GetPlayerCharacter` 0)))
      (`|AIMoveTo` self (0.0 0.0 0.0) _aswarrior_character_bp 1000.0))))

(event `Check_Player_Distance`
  ;[1 1 1] Check_Player Distance
  (bind _aswarrior_character_bp (cast `/Game/Fantasy_RPG_Game/Blueprints/Warrior/Warrior_Character_BP` (`GameplayStatics.GetPlayerCharacter` 0)))
  (switch `int` (`KismetMathLibrary.RandomInteger` 2)
    (:`Default`
      (`self.Breath_Fire_On_The_Ground`))
    (:`0`
      ;[1 1 1] Randomly_Switch_Between_Call_Bite or Breath_Fire_While_Flying
      (if (< (`self.GetDistanceTo` _aswarrior_character_bp) 900.0)
        (`/Engine/EditorBlueprintResources/StandardMacros.DoOnce` false :!label _label_2
          (:`Completed`
            (switch `int` (`KismetMathLibrary.RandomInteger` 5)
              (:`Default`
                (`PrimitiveComponent.SetCollisionEnabled` (`self.CapsuleComponent`) "NoCollision")
                (`self.BreathFire_Flying`))
              (:`0`
                (`self.Dragon_Bite` :!label _label_3))
              (:`1`
                (goto _label_3))
              (:`2`
                (goto _label_3)))))))))

(event `Initialize`
  ;[1 1 1] Initialize
  (if (not (`self.Dead`))
    (`|ExecutionSequence`
      (:`then_0`
        (`self.Attach_Dragon_Bite_Box`)
        (`|ExecutionSequence`
          (:`then_0`
            (if (`self.Can_Attack`)
              (if (`self.Can_Follow_Player`)
                (`|ExecutionSequence`
                  (:`then_0`
                    (`|ExecutionSequence`
                      (:`then_0`
                        (`self.Follow_Player`))
                      (:`then_2`
                        (`self.Check_Player_Distance`))))
                  (:`then_1`
                    (`KismetSystemLibrary.Delay` 0.06)
                    (`self.Initialize`))))))
          (:`then_1`
            (`self.Player_Detection_Animation`))))
      (:`then_1`
        ;[1 1 1] Create_Dragon_Health_Widget
        (`/Engine/EditorBlueprintResources/StandardMacros.DoOnce` false
          (:`Completed`
            (bind _returnvalue (`|CreateWidget` "/Game/Fantasy_RPG_Game/Widgets/Last_Blood_Dragon_Health_Widget.Last_Blood_Dragon_Health_Widget_C"))))))))

(event `Breath_Fire_On_The_Ground`
  (bind _dragon_fire (`self.Dragon_Fire`))
  ;[1 1 1] Breath_Fire_Grounded
  (if (`self.Dead`)
    _
    (elif (< (`self.GetDistanceTo` (stale `Check_Player_Distance` _aswarrior_character_bp)) 5000.0)
      (if (`self.Breath_Fire_Flying`)
        _
        (elif (not (`self.Bite`))
          (`/Engine/EditorBlueprintResources/StandardMacros.DoOnce` false :!label _label_4
            (:`Completed`
              (`self.Look_At_Player`)
              (set `CharacterMovementComponent.MaxWalkSpeed` 0.0 (`self.CharacterMovement`))
              (set `self.Breath_Fire_Grounded` true)
              (`|ExecutionSequence`
                (:`then_0`
                  (`KismetSystemLibrary.Delay` 1.2)
                  (`ActorComponent.Activate` _dragon_fire true)
                  (`SceneComponent.K2_AttachToComponent` _dragon_fire (`self.Mesh`) "Fire_Socket_Grounded" "KeepRelative" "KeepRelative" "KeepRelative" true)
                  (`KismetSystemLibrary.Delay` 5.0)
                  (`ActorComponent.Deactivate` _dragon_fire)
                  (set `self.Can_Follow_Player` true)
                  (set `CharacterMovementComponent.MaxWalkSpeed` 600.0 (`self.CharacterMovement`))
                  (`self.Initialize`)
                  (`self.Reset_Do_once`)
                  (`KismetSystemLibrary.Delay` 15.0)
                  (`self.Reset_Do_Once_2`))
                (:`then_1`
                  (set `self.Can_Follow_Player` false)
                  (set `self.Can_Look_At_Player` false)
                  (`KismetSystemLibrary.Delay` 6.0)
                  (set `self.Breath_Fire_Grounded` false)
                  (set `self.Can_Look_At_Player` true))))))))))

(event `Reset_Do_Once_2`
  ;[1 1 1] Breath_Fire_Grounded
  (goto _label_4 :!via `Reset`))

(event `Player_Detection_Animation`
  ;[1 1 1] Play Player Detacted Animation (Once)
  (`/Engine/EditorBlueprintResources/StandardMacros.DoOnce` false
    (:`Completed`
      (set `self.Player_Detected` true)
      (`KismetSystemLibrary.Delay` 0.6)
      (`KismetSystemLibrary.Delay` 2.8)
      (set `self.Player_Detected` false)
      (set `self.Can_Attack` true)
      (`self.Initialize`))))

(event `Hit_By_Sword`
  ;[1 1 1] Reduce_Health_When_Dragon_Hit_By_Player
  (switch `int` (`KismetMathLibrary.RandomInteger` 2)
    (:`Default`
      (`GameplayStatics.PlaySound2D` "/Game/Fantasy_RPG_Game/Sound/Effects/stab2_A.stab2_A" 1.0 1.0 0.0 null null))
    (:`0`
      (`GameplayStatics.PlaySound2D` "/Game/Fantasy_RPG_Game/Sound/Effects/Stab1_A.Stab1_A" 1.0 1.0 0.0 null null)))
  (if (`self.Can_Be_Hit`)
    (bind _output_get (set `self.Dragon_Health` (- (`self.Dragon_Health`) 0.02)))
    (`/Engine/EditorBlueprintResources/StandardMacros.CompareFloat` _output_get 0.01 :!label _label_5
      (:`==`
        _)
      (:`<`
        _))
    (`self.Death`)))

(event `Look_At_Player`
  (bind (_returnvalue_roll _returnvalue_pitch _returnvalue_yaw) (`KismetMathLibrary.BreakRotator` (`KismetMathLibrary.FindLookAtRotation` (`self.K2_GetActorLocation`) (`self.K2_GetActorLocation` (`GameplayStatics.GetPlayerCharacter` 0)))))
  ;[1 1 1] Look_At_Player
  (if (`self.Dead`)
    _
    (elif (`self.Can_Look_At_Player`)
      (if (not (`self.Breath_Fire_Grounded`))
        (`self.K2_SetActorRotation` (`KismetMathLibrary.MakeRotator` 0.0 0.0 _returnvalue_yaw))))))

(event `Hit_By_Bomb`
  ;[1 1 1] Reduce_Health_When_Dragon_Hit_By_Player
  (set `self.Dragon_Health` (- (`self.Dragon_Health`) 0.05))
  (goto _label_5))

(event `Hit_By_Power_Attack`
  ;[1 1 1] Reduce_Health_When_Dragon_Hit_By_Player
  (set `self.Dragon_Health` (- (`self.Dragon_Health`) 0.08))
  (goto _label_5))

(event `self.Dragon_Bite_Collision_Box.OnComponentBeginOverlap`
  (params (OverlappedComponent :type "PrimitiveComponent Object Reference") (OtherActor :type "Actor Object Reference") (OtherComp :type "PrimitiveComponent Object Reference") (OtherBodyIndex :type Integer) (bFromSweep :type Boolean) (SweepResult :type "HitResult Structure (by ref)"))
  ;[1 1 1] Cast_Dragon_Bite_Damage_to_Player
  (bind _aswarrior_character_bp (cast `/Game/Fantasy_RPG_Game/Blueprints/Warrior/Warrior_Character_BP` OtherActor))
  (if (`self.Bite`)
    (`/Engine/EditorBlueprintResources/StandardMacros.DoOnce` false :!label _label_6
      (:`Completed`
        (`KismetSystemLibrary.Delay` 0.1)
        (`/Game/Fantasy_RPG_Game/Blueprints/Warrior/Warrior_Character_BP.Dragon_Bite_Damage` _aswarrior_character_bp)
        (`KismetSystemLibrary.Delay` 2.25)
        (`self.Reset_Bite`)))))

(event `Reset_Bite`
  ;[1 1 1] Cast_Dragon_Bite_Damage_to_Player
  (goto _label_6 :!via `Reset`))

(event `Spawn_Sparks`
  ;[1 1 1] Spawn_Sparks_(Once out of 8 random chances)
  (switch `int` (`KismetMathLibrary.RandomInteger` 8)
    (:`0`
      (`|SpawnActorFromClass` "/Game/Fantasy_RPG_Game/Blueprints/Blood_Dragon/Dragon_Fire_Sparks_BP.Dragon_Fire_Sparks_BP_C" (`KismetMathLibrary.MakeTransform` (stale `self.Dragon_Fire.OnParticleCollide` Location)) "Undefined" "OverrideRootScale" null null))))

(event `self.Dragon_Fire.OnParticleCollide`
  (params (EventName :type Name) (EmitterTime :type "Float (single-precision)") (ParticleTime :type Integer) (Location :type "Vector Structure") (Velocity :type "Vector Structure") (Direction :type "Vector Structure") (Normal :type "Vector Structure") (BoneName :type Name) (PhysMat :type "PhysicalMaterial Object Reference"))
  (bind _returnvalue (`GameplayStatics.GetPlayerCharacter` 0))
  ;[1 1 1] Check_Distance_Between_Fire_Particle_Collision_And_Player
  (`|ExecutionSequence`
    (:`then_0`
      (`self.Spawn_Sparks`))
    (:`then_1`
      (if (== Location (`SceneComponent.K2_GetComponentLocation` (`Character.CapsuleComponent` _returnvalue)) :`ErrorTolerance` (`self.Dragon_Fire_Range`))
        ;[1 1 1] Cast_Fire_Damage_To_Player
        (bind _aswarrior_character_bp (cast `/Game/Fantasy_RPG_Game/Blueprints/Warrior/Warrior_Character_BP` _returnvalue))
        (`/Game/Fantasy_RPG_Game/Blueprints/Warrior/Warrior_Character_BP.Dragon_Fire_Hit` _aswarrior_character_bp)))))

(event `Death`
  ;[1 1 1] Death
  (set `self.Can_Be_Hit` false)
  (set `self.Player_Detected` true)
  (`KismetSystemLibrary.Delay` 3.2)
  (set `self.Player_Detected` false)
  (set `self.Dead` true)
  (set `self.Can_Follow_Player` false)
  (set `self.Bite` false)
  (set `self.Breath_Fire_Flying` false)
  (set `self.Breath_Fire_Grounded` false)
  (set `self.Can_Look_At_Player` false)
  (`CharacterMovementComponent.SetMovementMode` (`self.CharacterMovement`) "MOVE_Walking" 0)
  ;[1 1 1] Give_Player_1000XP
  (bind _aswarrior_character_bp (cast `/Game/Fantasy_RPG_Game/Blueprints/Warrior/Warrior_Character_BP` (`GameplayStatics.GetPlayerCharacter` 0)))
  (set `/Game/Fantasy_RPG_Game/Blueprints/Warrior/Warrior_Character_BP.XP_POINTS` (+ (`/Game/Fantasy_RPG_Game/Blueprints/Warrior/Warrior_Character_BP.XP_POINTS` _aswarrior_character_bp) 1000.0) _aswarrior_character_bp)
  ;[1 1 1] Hide_Dragon_Health
  (`Widget.RemoveFromParent` (stale `Initialize` _returnvalue))
  ;[1 1 1] Rag_Doll
  (`PrimitiveComponent.SetSimulatePhysics` (`self.Mesh`) true)
  (`PrimitiveComponent.SetCollisionEnabled` (`self.CapsuleComponent`) "NoCollision"))

(fn `UserConstructionScript`)